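; BP_Singleton1 is a save manager that persists collected coins per level, using the current level name as the save slot.
; SaveGame loads or creates an SG_bp, overwrites its PickedUpCoins with AlreadyCollectedObjects and writes it back.
; LoadGame waits briefly, clears AlreadyCollectedObjects without refilling it, then destroys each actor in the saved PickedUpCoins.
; DeleteSave removes the level's slot, and all three events print debug status.
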(event Custom|SaveGame
  ;[1 0.1323 0.2021] SaveGame
  (Development|PrintString "StartingSave")
  (bind _returnvalue (Game|GetCurrentLevelName true))
  (bind _returnvalue_2 (SaveGame|DoesSaveGameExist _returnvalue))
  (if _returnvalue_2
    (bind _returnvalue_3 (SaveGame|LoadGamefromSlot _returnvalue))
    (Variables|Default|SetSaverSubclass _returnvalue_3)
    (else
      (bind _returnvalue_4 (SaveGame|CreateSaveGameObject "/Game/Blueprints/SG_bp.SG_bp_C"))
      (Variables|Default|SetSaverSubclass _returnvalue_4)))
  (bind _assg_bp (Utilities|Casting|CastToSG_bp (Variables|Default|GetSaverSubclass)))
  (Variables|/Game/Blueprints/SG_bp.SG_bp_C|SetPickedUpCoins _assg_bp (Variables|Default|GetAlreadyCollectedObjects))
  (bind _returnvalue_5 (Game|GetCurrentLevelName true))
  (SaveGame|SaveGametoSlot _assg_bp _returnvalue_5)
  (Development|PrintString "SaveSuccessfull"))

(event Custom|LoadGame
  ;[0 0.4171 1] LoadGame
  (Utilities|FlowControl|Delay 0.2)
  (bind _returnvalue (Game|GetCurrentLevelName true))
  (Utilities|Array|Clear (Variables|Default|GetAlreadyCollectedObjects))
  (Development|PrintString (Utilities|String|Append "StartingLoadinLevel:  " _returnvalue ",WishMeLuck"))
  (bind _returnvalue_2 (SaveGame|DoesSaveGameExist _returnvalue))
  (if _returnvalue_2
    (bind _returnvalue_3 (SaveGame|LoadGamefromSlot _returnvalue))
    (bind _assg_bp (Utilities|Casting|CastToSG_bp _returnvalue_3))
    (Variables|Default|SetAs%20SG%20Bp _assg_bp)
    (for _array_element (Variables|/Game/Blueprints/SG_bp.SG_bp_C|GetPickedUpCoins _assg_bp)
      (Actor|DestroyActor _array_element))
    (else
      (Development|PrintString "SaveGameDoesNotExist"))))

(event Custom|DeleteSave
  (Development|PrintString "DeleteSave")
  (bind _returnvalue (Game|GetCurrentLevelName true))
  (bind _returnvalue_2 (SaveGame|DoesSaveGameExist _returnvalue))
  (if _returnvalue_2
    (SaveGame|DeleteGameinSlot _returnvalue)
    (Development|PrintString "SaveDeleted")
    (else
      (Development|PrintString "NoSaveGameExists"))))